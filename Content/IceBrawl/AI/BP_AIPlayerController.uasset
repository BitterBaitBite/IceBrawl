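; AI controller for computer-controlled players in IceBrawl, driven by the BT_AIPlayer behavior tree and BB_AIPlayer blackboard.
; On BeginPlay it stores the X and Y of the first actor tagged "Platform" as the arena center, then starts the tree.
; The tree does not run if no such actor exists.
; An ActivatePowerUp event, meant for animation notifies, sets the TriggerAbility blackboard flag.
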(event Custom|ActivatePowerUp
  ;[1 1 1] Activate powerup when animation notifies
  (AI|Components|Blackboard|SetValueasBool (AI|GetBlackboard 0) (Variables|Default|GetTriggerAbility) true))

(event EventBeginPlay
  (bind _blackboardcomponent (Class|AIController|UseBlackboard "/Game/IceBrawl/AI/BB_AIPlayer.BB_AIPlayer"))
  (bind _outactors (Actor|GetAllActorswithTag "Platform"))
  (if (> (Utilities|Array|Length _outactors) 0)
    (AI|Components|Blackboard|SetValueasVector _blackboardcomponent (Variables|Default|GetArenaCenterPosition) (Math|Vector|MakeVector (.x (Transformation|GetActorLocation (Utilities|Array|Get(acopy) _outactors))) (.y (Transformation|GetActorLocation (Utilities|Array|Get(acopy) _outactors))) 0.0))
    (AI|RunBehaviorTree "/Game/IceBrawl/AI/BT_AIPlayer.BT_AIPlayer")))

(fn ConstructionScript)