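; Game mode for IceBrawl that sets up a two-player penguin match and keeps score.
; BeginPlay shows the score widget, adds an AI or local second player per the game instance's UseIA flag, reskins it and creates energy bars.
; While CheckScore is set, Tick polls characters for deaths, credits the opponent in the game instance and refreshes the score.
; Reaching the max score shows a timed winner widget; level-loading nodes are unconnected.
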(event EventTick
  (params (DeltaSeconds :type Float%20%28single-precision%29))
  (Variables|Default|SetPlayerDeadIndex -1)
  (bind _asbp_game_instance (Utilities|Casting|CastToBP_GameInstance (Game|GetGameInstance)))
  (if (Variables|/Game/IceBrawl/Blueprints/BP_GameInstance.BP_GameInstance_C|GetCheckScore _asbp_game_instance)
    (bind _outactors (Actor|GetAllActorsOfClass "/Game/IceBrawl/Blueprints/BP_PlayerCharacter.BP_PlayerCharacter_C"))
    (bind (_array_element _array_index) (Utilities|Array|ForEachLoopwithBreak _outactors :!label _label)
      (:LoopBody
        (if (Variables|/Game/IceBrawl/Blueprints/BP_PlayerCharacter.BP_PlayerCharacter_C|GetIsDead _array_element)
          (Variables|Default|SetPlayerDeadIndex _array_index)
          (Variables|/Game/IceBrawl/Blueprints/BP_PlayerCharacter.BP_PlayerCharacter_C|SetIsDead _array_element false)
          (goto _label Break)))
      (:Completed
        (Utilities|FlowControl|Sequence
          (:then_0
            ;[1 1 1] Increments Score
            (bind _asbp_game_instance_2 (Utilities|Casting|CastToBP_GameInstance (Game|GetGameInstance)))
            (if (!= (Variables|Default|GetPlayerDeadIndex) -1)
              (if (== (Variables|Default|GetPlayerDeadIndex) 0)
                (Math|Integer|IncrementInt (Variables|/Game/IceBrawl/Blueprints/BP_GameInstance.BP_GameInstance_C|GetPlayer2Score _asbp_game_instance_2))
                (elif (== (Variables|Default|GetPlayerDeadIndex) 1)
                  (Math|Integer|IncrementInt (Variables|/Game/IceBrawl/Blueprints/BP_GameInstance.BP_GameInstance_C|GetPlayer1Score _asbp_game_instance_2))))))
          (:then_1
            (bind _aswp_score (Utilities|Casting|CastToWP_Score (Variables|Default|GetScoreWidget)))
            (Default|SetPlayer1Score _aswp_score (Variables|/Game/IceBrawl/Blueprints/BP_GameInstance.BP_GameInstance_C|GetPlayer1Score _asbp_game_instance_2))
            (Default|SetPlayer2Score _aswp_score (Variables|/Game/IceBrawl/Blueprints/BP_GameInstance.BP_GameInstance_C|GetPlayer2Score _asbp_game_instance_2)))
          (:then_2
            ;[1 1 1] Check if there is a winner
            (if (>= (Variables|/Game/IceBrawl/Blueprints/BP_GameInstance.BP_GameInstance_C|GetPlayer1Score _asbp_game_instance_2) (Variables|/Game/IceBrawl/Blueprints/BP_GameInstance.BP_GameInstance_C|GetPlayerMaxScore _asbp_game_instance_2))
              (bind _returnvalue (UserInterface|CreateWidget "/Game/IceBrawl/Widgets/WP_Winner.WP_Winner_C" (Game|GetPlayerController 0)))
              (UserInterface|Viewport|AddtoViewport _returnvalue 0)
              (Default|SetWinner _returnvalue "PLAYER1")
              (Utilities|FlowControl|Delay 5.0)
              (Widget|RemovefromParent _returnvalue)
              (elif (>= (Variables|/Game/IceBrawl/Blueprints/BP_GameInstance.BP_GameInstance_C|GetPlayer2Score _asbp_game_instance_2) (Variables|/Game/IceBrawl/Blueprints/BP_GameInstance.BP_GameInstance_C|GetPlayerMaxScore _asbp_game_instance_2))
                (bind _returnvalue_2 (UserInterface|CreateWidget "/Game/IceBrawl/Widgets/WP_Winner.WP_Winner_C"))
                (UserInterface|Viewport|AddtoViewport _returnvalue_2 0)
                (Default|SetWinner _returnvalue_2 "PLAYER2")
                (Utilities|FlowControl|Delay 5.0)
                (Widget|RemovefromParent _returnvalue_2)))))))))

(event EventBeginPlay
  (bind _returnvalue (Game|GetPlayerController 0))
  (bind _returnvalue_2 (Game|GetPlayerCharacter 1))
  (Input|SetInputModeGameOnly _returnvalue false)
  (bind _returnvalue_3 (UserInterface|CreateWidget "/Game/IceBrawl/Widgets/WP_Score.WP_Score_C" _returnvalue))
  (bind _output_get (Variables|Default|SetScoreWidget _returnvalue_3))
  (UserInterface|Viewport|AddtoViewport _output_get 0)
  (bind _asbp_game_instance (Utilities|Casting|CastToBP_GameInstance (Game|GetGameInstance)))
  (Variables|Default|SetAIPlayer (Variables|/Game/IceBrawl/Blueprints/BP_GameInstance.BP_GameInstance_C|GetUseIA _asbp_game_instance))
  (if (Variables|Default|GetAIPlayer)
    (Class|GameplayStatics|CreatePlayer -1 false)
    (bind _returnvalue_4 (Game|SpawnActorfromClass "/Game/IceBrawl/Blueprints/BP_PlayerCharacter.BP_PlayerCharacter_C" (Math|Conversions|ToTransform(Vector) (Variables|Default|GetPlayer2StartPosition)) "Undefined" "MultiplyWithRoot" 0 0))
    (Rendering|Material|SetMaterial (Variables|/Script/Engine.Character|GetMesh _returnvalue_4) 2 "/Game/IceBrawl/Mannequins/Pinguins/Models/Materials/MI_BadPenguin.MI_BadPenguin")
    (Rendering|Material|SetMaterial (Variables|/Script/Engine.Character|GetMesh _returnvalue_4) 1 "/Game/IceBrawl/Mannequins/Pinguins/Models/Materials/MI_BadHat.MI_BadHat")
    (bind _returnvalue_5 (Game|SpawnActorfromClass "/Game/IceBrawl/AI/BP_AIPlayerController.BP_AIPlayerController_C" (Transformation|GetActorTransform _returnvalue_4) "Undefined" "MultiplyWithRoot" 0 0))
    (Pawn|Possess _returnvalue_5 _returnvalue_4)
    (bind _returnvalue_6 (UserInterface|CreateWidget "/Game/IceBrawl/Widgets/EnergyBars.EnergyBars_C"))
    (UserInterface|Viewport|AddtoViewport _returnvalue_6 0)
    (bind _asenergy_bars (Utilities|Casting|CastToEnergyBars _returnvalue_6))
    (Default|Initialize _asenergy_bars _returnvalue_5)
    (else
      (bind _returnvalue_7 (Class|GameplayStatics|CreatePlayer -1))
      (Transformation|SetActorLocation (Pawn|GetControlledPawn _returnvalue_7) (Variables|Default|GetPlayer2StartPosition) false false)
      (Rendering|Material|SetMaterial (Variables|/Script/Engine.Character|GetMesh _returnvalue_2) 2 "/Game/IceBrawl/Mannequins/Pinguins/Models/Materials/MI_BadPenguin.MI_BadPenguin")
      (Rendering|Material|SetMaterial (Variables|/Script/Engine.Character|GetMesh _returnvalue_2) 1 "/Game/IceBrawl/Mannequins/Pinguins/Models/Materials/MI_BadHat.MI_BadHat")
      (bind _returnvalue_8 (UserInterface|CreateWidget "/Game/IceBrawl/Widgets/EnergyBars.EnergyBars_C"))
      (UserInterface|Viewport|AddtoViewport _returnvalue_8 0)
      (bind _asenergy_bars_2 (Utilities|Casting|CastToEnergyBars _returnvalue_8))
      (Default|Initialize _asenergy_bars_2 _returnvalue_7))))

(fn ConstructionScript)