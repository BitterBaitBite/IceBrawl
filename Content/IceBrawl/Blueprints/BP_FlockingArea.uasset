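; BP_FlockingArea is an IceBrawl actor that defines a flocking area by a center point and radius.
; On BeginPlay it stores its location as Center and scales a flattened Preview mesh to the radius's diameter, with a minimum size clamp.
; The ShowPreview flag controls whether that mesh is visible in game.
; The Blueprint contains no flocking logic, and its construction script is empty.
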(event EventBeginPlay
  (bind _radius (Variables|Default|GetRadius))
  (bind _returnvalue (/ _radius 1e+02))
  (bind _returnvalue_2 (Math|Float|Max(Float) _returnvalue 1.0))
  (bind _returnvalue_3 (* _returnvalue_2 2.0))
  ;[1 1 1] Set center variable
  (Variables|Default|SetCenter (Transformation|GetActorLocation))
  ;[1 1 1] Set preview mesh
  (Transformation|SetRelativeScale3D (Variables|Default|GetPreview) (Math|Vector|MakeVector _returnvalue_3 _returnvalue_3 0.0))
  ;[1 1 1] Set preview visibility
  (Development|SetHiddeninGame (Variables|Default|GetPreview) (not (Variables|Default|GetShowPreview)) false))

(fn ConstructionScript)