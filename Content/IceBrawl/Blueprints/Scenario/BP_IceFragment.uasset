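; BP_IceFragment is a physics-driven chunk of ice that floats in water volumes.
; On BeginPlay it applies the configured ice mesh and a large random yaw torque in either direction.
; Overlapping a water PhysicsVolume turns floating on and records the top of its bounds as the surface height; leaving turns it off.
; While floating, Tick applies simple spring-like buoyancy: a vertical force proportional to distance from the surface, scaled by mass.
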(event OnComponentBeginOverlap(Mesh)
  (params (OverlappedComponent :type Primitive%20Component%20Object%20Reference) (OtherActor :type Actor%20Object%20Reference) (OtherComp :type Primitive%20Component%20Object%20Reference) (OtherBodyIndex :type Integer) (bFromSweep :type Boolean) (SweepResult :type Hit%20Result%20Structure%20%28by%20ref%29))
  (bind _asphysics_volume (Utilities|Casting|CastToPhysicsVolume OtherActor))
  (if (Variables|/Script/Engine.PhysicsVolume|GetbWaterVolume _asphysics_volume)
    (Variables|Default|SetIsFloating true)
    (Variables|Default|SetWaterHeight (+ (.z (.Origin (Collision|GetActorBounds _asphysics_volume false false))) (.z (.BoxExtent (Collision|GetActorBounds _asphysics_volume false false)))))))

(event OnComponentEndOverlap(Mesh)
  (params (OverlappedComponent :type Primitive%20Component%20Object%20Reference) (OtherActor :type Actor%20Object%20Reference) (OtherComp :type Primitive%20Component%20Object%20Reference) (OtherBodyIndex :type Integer))
  (bind _asphysics_volume (Utilities|Casting|CastToPhysicsVolume OtherActor))
  (if (Variables|/Script/Engine.PhysicsVolume|GetbWaterVolume _asphysics_volume)
    (Variables|Default|SetIsFloating false)))

(event EventTick
  (params (DeltaSeconds :type Float%20%28single-precision%29))
  (bind _mesh (Variables|Default|GetMesh))
  (if (Variables|Default|GetIsFloating)
    (Physics|AddForce _mesh (Math|Vector|MakeVector 0.0 0.0 (* (* (- (Variables|Default|GetWaterHeight) (.z (Transformation|GetWorldLocation _mesh))) (Variables|Default|GetFloatabilityFactor)) (* (Physics|GetMass _mesh) 9.8))) "None" false)))

(event EventBeginPlay
  (Components|StaticMesh|SetStaticMesh (Variables|Default|GetMesh) (Variables|Default|GetIceMesh))
  (Class|PrimitiveComponent|AddTorqueinDegrees (Variables|Default|GetMesh) (Math|Vector|MakeVector 0.0 0.0 (* (Math|Random|RandomFloatinRange -1.0 1.0) 1e+08)) "None" false))

(fn ConstructionScript)