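; Physics prop for IceBrawl that falls toward a spherical water volume and floats on it.
; BeginPlay sets the mesh, takes the first BP_WaterSphereVolume as gravity center and picks a random yaw rate.
; Each tick, a mass-scaled inward radial force fakes gravity; while floating, an outward linear-falloff force adds buoyancy alongside a slow spin.
; Mesh overlaps with water volumes toggle floating, updating center and radius on entry.
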(event OnComponentBeginOverlap(Mesh)
  (params (OverlappedComponent :type Primitive%20Component%20Object%20Reference) (OtherActor :type Actor%20Object%20Reference) (OtherComp :type Primitive%20Component%20Object%20Reference) (OtherBodyIndex :type Integer) (bFromSweep :type Boolean) (SweepResult :type Hit%20Result%20Structure%20%28by%20ref%29))
  (bind _asbp_water_sphere_volume (Utilities|Casting|CastToBP_WaterSphereVolume OtherActor))
  (Variables|Default|SetIsFloating true)
  (Variables|Default|SetCenterOfWaterVolume (.Origin (Collision|GetComponentBounds (Variables|/Script/Engine.TriggerBase|GetCollisionComponent _asbp_water_sphere_volume))))
  (Variables|Default|SetWaterVolumeRadius (.SphereRadius (Collision|GetComponentBounds (Variables|/Script/Engine.TriggerBase|GetCollisionComponent _asbp_water_sphere_volume)))))

(event OnComponentEndOverlap(Mesh)
  (params (OverlappedComponent :type Primitive%20Component%20Object%20Reference) (OtherActor :type Actor%20Object%20Reference) (OtherComp :type Primitive%20Component%20Object%20Reference) (OtherBodyIndex :type Integer))
  (Utilities|Casting|CastToBP_WaterSphereVolume OtherActor)
  (Variables|Default|SetIsFloating false))

(event EventTick
  (params (DeltaSeconds :type Float%20%28single-precision%29))
  (bind _mesh (Variables|Default|GetMesh))
  ;[1 1 1] Gravity force
  (Utilities|IsValid (Variables|Default|GetDefaultWaterVolume)
    (:Is%20Valid
      (Physics|AddRadialForce (Variables|Default|GetMesh) (Variables|Default|GetCenterOfWaterVolume) (+ (Variables|Default|GetWaterVolumeRadius) 1e+04) (* (Physics|GetMass (Variables|Default|GetMesh)) -9.8e+03) "RIF_Constant" false)
      ;[1 1 1] Floating force
      (if (Variables|Default|GetIsFloating)
        (Physics|AddRadialForce _mesh (Variables|Default|GetCenterOfWaterVolume) (+ (Variables|Default|GetWaterVolumeRadius) 5e+01) (* 5.0 (* (* (Physics|GetMass _mesh) (Variables|Default|Getgravity)) (Variables|Default|Getcm/s))) "RIF_Linear" false)
        ;[1 1 1] Set the random rotation
        (Transformation|AddRelativeRotation (Variables|Default|GetMesh) (Math|Rotator|MakeRotator 0.0 0.0 (/ (Variables|Default|GetRandomRotationZ) 1e+01)) false false)))))

(event EventBeginPlay
  (bind _rotationrate (Variables|Default|GetRotationRate))
  ;[1 1 1] Mesh init
  (Components|StaticMesh|SetStaticMesh (Variables|Default|GetMesh) (Variables|Default|GetIceMesh))
  ;[1 1 1] Set default water volume for fake gravity
  (bind _outactors (Actor|GetAllActorsOfClass "/Game/IceBrawl/Blueprints/Scenario/BP_WaterSphereVolume.BP_WaterSphereVolume_C"))
  (bind _output_get (Variables|Default|SetDefaultWaterVolume (Utilities|Array|Get(acopy) _outactors)))
  (Variables|Default|SetCenterOfWaterVolume (.Origin (Collision|GetComponentBounds (Variables|/Script/Engine.TriggerBase|GetCollisionComponent _output_get))))
  (Variables|Default|SetWaterVolumeRadius (.SphereRadius (Collision|GetComponentBounds (Variables|/Script/Engine.TriggerBase|GetCollisionComponent _output_get))))
  ;[1 1 1] Get a random rotation based on rate
  (Variables|Default|SetRandomRotationZ (Math|Random|RandomFloatinRange (* _rotationrate -1.0) _rotationrate)))

(fn ConstructionScript)