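; Boids-style schooling fish that swims as a physics-driven mesh inside a spherical FlockingArea.
; Each tick it sums distance-weighted alignment, cohesion and separation from all other BP_FlockingFish with a timer-randomized steer and a pull toward the center near the edge.
; The resulting direction drives AddForce, and the mesh rotates to face its velocity.
; Outside the area, outward velocity and direction are reflected back inward.
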(event EventBeginPlay
  (bind _fishmesh (Variables|Default|GetFishMesh))
  (bind _fishmodel (Variables|Default|GetFishModel))
  ;[1 1 1] Set static mesh
  (if (== (Variables|Default|GetFishModel) _fishmesh)
    _
    (else
      (Components|StaticMesh|SetStaticMesh (Variables|Default|GetFishModel) _fishmesh)))
  ;[1 1 1] Set mesh scale
  (Transformation|SetRelativeScale3D _fishmodel (* (Variables|/Script/Engine.SceneComponent|GetRelativeScale3D _fishmodel) (Variables|Default|GetMeshScale)))
  ;[1 1 1] Initial random direction
  (Variables|Default|SetDirection (Math|Random|RandomUnitVector))
  ;[1 1 1] Get all flocking entities
  (bind _outactors (Actor|GetAllActorsOfClass "BP_FlockingFish_C"))
  (bind _output_get (Variables|Default|SetFlockingArray _outactors))
  (Utilities|Array|RemoveItem _output_get self)
  ;[1 1 1] Set a timed function to calc steer direction
  (Utilities|Time|SetTimerbyFunctionName 0 "CalcSteerDirection" 1.5 true)
  (CallFunction|CalcSteerDirection))

(event EventTick
  (params (DeltaSeconds :type Float%20%28single-precision%29))
  (Utilities|IsValid (Variables|Default|GetFlockingArea)
    (:Is%20Valid
      (CallFunction|ResetForces)
      (for _array_element (Variables|Default|GetFlockingArray)
        ;[1 1 1] Calc flocking forces per instance
        (CallFunction|CalcAlignment _array_element)
        (CallFunction|CalcCohesion _array_element)
        (CallFunction|CalcSeparation _array_element))
      ;[1 1 1] Stay inside area
      (bind _isinsidearea (CallFunction|IsInsideArea))
      (if _isinsidearea
        (CallFunction|SumForces)
        ;[1 1 1] Forward force
        (Physics|AddForce (Variables|Default|GetFishModel) (* (Variables|Default|GetDirection) (Variables|Default|GetLinearForceFactor)) "None" false)
        ;[1 1 1] Rotate to match velocity
        (CallFunction|RotateFishTowardsVelocity)
        (else
          (CallFunction|InvertDirectionTowardsArea))))))

(fn ConstructionScript)

(fn IsInsideArea
  (bind _flockingarea (Variables|Default|GetFlockingArea))
  (return (<= (Math|Vector|VectorLength (- (Variables|/Game/IceBrawl/Blueprints/Flocking/BP_FlockingArea.BP_FlockingArea_C|GetCenter _flockingarea) (Transformation|GetWorldLocation (Variables|Default|GetFishModel)))) (Variables|/Game/IceBrawl/Blueprints/Flocking/BP_FlockingArea.BP_FlockingArea_C|GetRadius _flockingarea))))

(fn InvertDirectionTowardsArea
  (bind _fishmodel (Variables|Default|GetFishModel))
  (bind _flockingarea (Variables|Default|GetFlockingArea))
  (bind _fishmodel_2 (Variables|Default|GetFishModel))
  (bind _returnvalue (Transformation|GetComponentVelocity _fishmodel))
  (bind _returnvalue_2 (Transformation|GetWorldLocation _fishmodel_2))
  (bind _center (Variables|/Game/IceBrawl/Blueprints/Flocking/BP_FlockingArea.BP_FlockingArea_C|GetCenter _flockingarea))
  (bind _returnvalue_3 (- _returnvalue_2 _center))
  (bind _returnvalue_4 (Math|Vector|Normalize _returnvalue_3))
  (bind _returnvalue_5 (Math|Vector|DotProduct _returnvalue _returnvalue_4))
  (if (> _returnvalue_5 0.0)
    (Physics|SetPhysicsLinearVelocity (Variables|Default|GetFishModel) (+ _returnvalue (* (* _returnvalue_5 _returnvalue_4) -2)) false "None")
    (bind _output_get (Variables|Default|SetDirection (+ (* (* _returnvalue_4 (Math|Vector|DotProduct _returnvalue_4 (Variables|Default|GetDirection))) -2) (Variables|Default|GetDirection))))))

(fn RotateFishTowardsVelocity
  (bind _fishmodel (Variables|Default|GetFishModel))
  (Transformation|SetRelativeRotation _fishmodel (Math|Rotator|CombineRotators (Math|Conversions|RotationFromXVector (Transformation|GetComponentVelocity _fishmodel)) "0.000000,-90.000000,0.000000") false false))

(fn ResetForces
  (Variables|Default|SetAlignmentDirection "0, 0, 0")
  (Variables|Default|SetCohesionDirection "0, 0, 0")
  (Variables|Default|SetSeparationDirection "0, 0, 0"))

(fn CalcAlignment
  (params (FlockingEntity :type BP%20Flocking%20Fish%20Object%20Reference))
  (Variables|Default|SetAlignmentDirection (+ (* (Variables|BP_FlockingFish_C|GetDirection FlockingEntity) (Math|Float|MapRangeClamped (Math|Vector|VectorLength (- (Transformation|GetWorldLocation (Variables|Default|GetFishModel)) (Transformation|GetWorldLocation (Variables|BP_FlockingFish_C|GetFishModel FlockingEntity)))) 0.0 (Variables|Default|GetAlignmentRadius) 1.0 0.0)) (Variables|Default|GetAlignmentDirection))))

(fn SumForces
  (bind _output_get (Variables|Default|SetDirection (Math|Vector|Normalize (+ (* (Variables|Default|GetDirection) (Variables|Default|GetLinearForceFactor)) (* (Variables|Default|GetAlignmentDirection) (Variables|Default|GetAlignmentFactor)) (* (Variables|Default|GetCohesionDirection) (Variables|Default|GetCohesionFactor)) (* (Variables|Default|GetSeparationDirection) (Variables|Default|GetSeparationFactor)) (* (Variables|Default|GetSteerDirection) (Variables|Default|GetSteeringFactor))))))
  (bind _forcetowardstarget (CallFunction|CalcForceTowardsCenter))
  (Variables|Default|SetDirection (Math|Vector|Normalize (+ _forcetowardstarget _output_get))))

(fn CalcForceTowardsCenter
  (bind _fishmodel (Variables|Default|GetFishModel))
  (bind _flockingarea (Variables|Default|GetFlockingArea))
  (bind _flockingarea_2 (Variables|Default|GetFlockingArea))
  (bind _returnvalue (Transformation|GetWorldLocation _fishmodel))
  (bind _center (Variables|/Game/IceBrawl/Blueprints/Flocking/BP_FlockingArea.BP_FlockingArea_C|GetCenter _flockingarea))
  (bind _radius (Variables|/Game/IceBrawl/Blueprints/Flocking/BP_FlockingArea.BP_FlockingArea_C|GetRadius _flockingarea_2))
  (bind _returnvalue_2 (- _center _returnvalue))
  (return (* (* (Math|Vector|Normalize _returnvalue_2) (Math|Float|MapRangeClamped (Math|Vector|VectorLength _returnvalue_2) (* _radius (Variables|Default|GetTowardsCenterRadius)) _radius 0.0 1.0)) (Variables|Default|GetTowardsCenterFactor))))

(fn CalcCohesion
  (params (self2 :type BP%20Flocking%20Fish%20Object%20Reference))
  (bind _fishmodel (Variables|BP_FlockingFish_C|GetFishModel self2))
  (bind _fishmodel_2 (Variables|Default|GetFishModel))
  (bind _returnvalue (Transformation|GetWorldLocation _fishmodel))
  (bind _returnvalue_2 (Transformation|GetWorldLocation _fishmodel_2))
  (bind _returnvalue_3 (- _returnvalue _returnvalue_2))
  (Variables|Default|SetCohesionDirection (+ (* (Math|Vector|Normalize _returnvalue_3) (Math|Float|MapRangeClamped (Math|Vector|VectorLength _returnvalue_3) 0.0 (Variables|Default|GetCohesionRadius) 1.0 0.0)) (Variables|Default|GetCohesionDirection))))

(fn CalcSeparation
  (params (self2 :type BP%20Flocking%20Fish%20Object%20Reference))
  (bind _fishmodel (Variables|BP_FlockingFish_C|GetFishModel self2))
  (bind _fishmodel_2 (Variables|Default|GetFishModel))
  (bind _returnvalue (Transformation|GetWorldLocation _fishmodel))
  (bind _returnvalue_2 (Transformation|GetWorldLocation _fishmodel_2))
  (bind _returnvalue_3 (- _returnvalue _returnvalue_2))
  (Variables|Default|SetSeparationDirection (+ (* (Math|Vector|Normalize (* _returnvalue_3 -1)) (Math|Float|MapRangeClamped (Math|Vector|VectorLength _returnvalue_3) 0.0 (Variables|Default|GetSeparationRadius) 1.0 0.0)) (Variables|Default|GetSeparationDirection))))

(fn CalcSteerDirection
  (bind _fishmodel (Variables|Default|GetFishModel))
  (bind _steeringangle (Variables|Default|GetSteeringAngle))
  (bind _relativerotation (Variables|/Script/Engine.SceneComponent|GetRelativeRotation _fishmodel))
  (bind _output_get (Variables|Default|SetSteerDirection (Math|Vector|GetForwardVector (Math|Rotator|MakeRotator (.roll _relativerotation) (.pitch _relativerotation) (+ (.yaw _relativerotation) (Math|Random|RandomFloatinRange (* _steeringangle -1) _steeringangle)))))))